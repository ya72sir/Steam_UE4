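; Base weapon actor that fires projectile ammo from a transform its owner supplies, with server-authoritative ammo, fire-rate delay and timed reload.
; Fire requests route to the server, which spawns the projectile with damage and instigator, multicasts the owner's attack animation, and reloads when ammo runs out.
; State changes flip a boolean whose RepNotify passes the weapon to the instigator's PS_Gameplay player state.
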(event `self.ReceiveBeginPlay`
  (`/Engine/EditorBlueprintResources/ActorMacros.Switch Has Authority`
    (:`Authority`
      (set `self.Ammo_Current` (`self.Ammo_Max`))
      (`self.UpdateInfoState`))))

(event `ServerFire`
  (params (TransformSpawnAmmo :type "Transform Structure"))
  ;[1 1 1] Fire
  (set `self.TransformSpawnAmmo` TransformSpawnAmmo)
  (`/Engine/EditorBlueprintResources/ActorMacros.Switch Has Authority` :!label _label
    (:`Authority`
      (if (`self.WeaponWaitCurrentAction`)
        _
        (elif (> (`self.Ammo_Current`) 0)
          (`|SpawnActorFromClass` (`self.Ammo`) (`self.TransformSpawnAmmo`) "AlwaysSpawn" "OverrideRootScale" self (`self.Damage`) 3.0 (`self.GetInstigator`))
          (set `self.FireActive?` false)
          (`/Engine/EditorBlueprintResources/StandardMacros.DecrementInt` (`self.Ammo_Current`)
            (:`  `
              (`self.UpdateState`)
              ;;[1 1 1] Weapon Animmontage! Play montage
              (`/Game/Sir/Core/Blueprints/Characters/0_Base.PlayAnimAttack_Multicast` (cast `/Game/Sir/Core/Blueprints/Characters/0_Base` (`self.GetOwner`) :!pure true))
              (`KismetSystemLibrary.Delay` (`self.TimeFire`))
              (set `self.FireActive?` true)
              (if (<= (`self.Ammo_Current`) 0)
                ;[1 1 1] Reload
                (set `self.Reload?` true :!label _label_2)
                (`self.UpdateState`)
                (set `self.WeaponWaitCurrentAction` true)
                (`KismetSystemLibrary.Delay` (`self.TimeReload`))
                (set `self.Ammo_Current` (`self.Ammo_Max`))
                (set `self.Reload?` false)
                (set `self.WeaponWaitCurrentAction` false)
                (`self.UpdateState`))))
          (else
            (goto _label_2)))))
    (:`Remote`
      (`self.ServerFire` (`self.TransformSpawnAmmo`)))))

(event `Fire`
  ;[1 1 1] Fire
  (if (`self.FireActive?`)
    (bind _ammo (message `/Game/Sir/Core/Blueprints/Interfaces/BPI_Character.bpiGetTransformAmmo` (`self.GetOwner`)))
    (set `self.TransformSpawnAmmo` _ammo)
    (goto _label)))

(event `UpdateInfoState`
  (bind _returnvalue (`self.GetInstigatorController` (`self.GetOwner`)))
  ;[1 1 1] Client - update State
  (`/Engine/EditorBlueprintResources/StandardMacros.IsValid` _returnvalue
    (:`Is Valid`
      (`/Game/Sir/Core/Blueprints/Gameplay/PS_Gameplay.UpdateState` (cast `/Game/Sir/Core/Blueprints/Gameplay/PS_Gameplay` (`Controller.PlayerState` _returnvalue) :!pure true) self))))

(fn `OnRep_UpdatePlayerState`
  (`self.UpdateInfoState`))

(fn `UserConstructionScript`
  (`StaticMeshComponent.SetStaticMesh` (`self.StaticMesh`) (`self.WeaponStaticMesh`)))