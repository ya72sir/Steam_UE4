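; Gameplay GameState that holds the battle timer and session info shown on the player's HUD.
; Events store the minutes, seconds and battle-end value, and replace the session info array.
; ShowInfoSession caches the player controller and visibility flag, then has the controller create or remove the session HUD.
; The InfoSession RepNotify refreshes that HUD through the cached controller while the flag is set.
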(event `UpdateBattleTime`
  (params (Minute :type Integer) (Seconde :type Integer) (`BattleEnd?` :type Boolean))
  (set `self.Min` Minute)
  (set `self.Sec` Seconde)
  (set `self.BattleEnd?` `BattleEnd?`))

(event `ShowInfoSession`
  (params (PlayerController :type "/Game/Sir/Core/Blueprints/Gameplay/PC_Gameplay Object Reference") (`ShowInfoAboutSession?` :type Boolean))
  (set `self.ShowInfoAboutSession?` `ShowInfoAboutSession?`)
  (bind _output_get (set `self.PlayerController` PlayerController))
  (`/Game/Sir/Core/Blueprints/Gameplay/PC_Gameplay.HUD_SessionInfo` _output_get (`self.InfoSession`) false))

(event `UpdateInfoAboutSession`
  (params (InfoSession :type "Array of Text"))
  (set `self.InfoSession` InfoSession))

(fn `OnRep_InfoSession`
  (bind _playercontroller (`self.PlayerController`)
    (:`then`
      (if (`self.ShowInfoAboutSession?`)
        (`/Game/Sir/Core/Blueprints/Gameplay/PC_Gameplay.HUD_SessionInfo` _playercontroller (`self.InfoSession`) true)))
    (:`else`)))

(fn `UserConstructionScript`)