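; Gameplay HUD Blueprint that creates and manages the player's on-screen widgets.
; Shortly after BeginPlay it registers itself on PC_Gameplay, then adds the aim and gameplay screen widgets.
; Events show the win/lose end screen and create, rebuild or remove the session info widget.
; Chat events create a hidden chat widget, toggle or disable it, and briefly reveal it for temporary messages.
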(event `self.ReceiveBeginPlay`
  (`KismetSystemLibrary.Delay` 0.2)
  (set `/Game/Sir/Core/Blueprints/Gameplay/PC_Gameplay.GameplayHUD` self (cast `/Game/Sir/Core/Blueprints/Gameplay/PC_Gameplay` (`self.GetOwningPlayerController`) :!pure true))
  (bind _returnvalue (`|CreateWidget` "/Game/Sir/UI/Gameplay/WB_Aim.WB_Aim_C"))
  (bind _output_get (set `self.WB_AIM` _returnvalue))
  (`UserWidget.AddToViewport` _output_get 0)
  (bind _returnvalue_2 (`|CreateWidget` "/Game/Sir/UI/Gameplay/WB_ScreenGameplay.WB_ScreenGameplay_C" (`self.PlayerController`)))
  (bind _output_get_2 (set `self.WB_ScreenGameplay` _returnvalue_2))
  (`UserWidget.AddToViewport` _output_get_2 0))

(event `ShowEndScreen`
  (params (`Win?` :type Boolean) (OwningPlayer :type "PlayerController Object Reference"))
  (bind _returnvalue (`|CreateWidget` "/Game/Sir/UI/Gameplay/WB_EndScreen.WB_EndScreen_C" OwningPlayer `Win?`))
  (`UserWidget.AddToViewport` _returnvalue 0))

(event `SessionInfo`
  (params (arrInfo :type "Array of Text") (UpdateInfo :type Boolean))
  (bind _wb_sessioninfo (`self.WB_SessionInfo`)
    (:`then`
      (`Widget.RemoveFromParent` _wb_sessioninfo)
      (set `self.WB_SessionInfo` null)
      (if UpdateInfo
        (bind _returnvalue (`|CreateWidget` "/Game/Sir/UI/Gameplay/WB_SessionInfo.WB_SessionInfo_C" null arrInfo :!label _label))
        (bind _output_get (set `self.WB_SessionInfo` _returnvalue))
        (`UserWidget.AddToViewport` _output_get 0)))
    (:`else`
      (goto _label))))

(event `SetupChat`
  (params (OwningPlayer :type "PlayerController Object Reference"))
  (bind _returnvalue (`|CreateWidget` "/Game/Sir/UI/AllLevels/wGameplayChat.wGameplayChat_C" OwningPlayer))
  (bind _output_get (set `self.WB_GameplayChat` _returnvalue))
  (`UserWidget.AddToViewport` _output_get 0)
  (`Widget.SetVisibility` _output_get "Hidden"))

(event `ToggleChat`
  (bind _wb_gameplaychat (`self.WB_GameplayChat`))
  (`Widget.SetVisibility` _wb_gameplaychat (select `bool` (`|EnumEquality` (`Widget.GetVisibility` _wb_gameplaychat) "Hidden") :`false` "Hidden" :`true` "Visible" :!type "ESlateVisibility Enum")))

(event `DisableChat`
  (if (`|EnumEquality` (`Widget.GetVisibility` (`self.WB_GameplayChat`)) "Visible")
    (`Widget.SetVisibility` (`self.WB_GameplayChat`) "Hidden")
    (bind _playercontroller (`self.PlayerController`)
      (:`then`
        (set `PlayerController.bShowMouseCursor` false _playercontroller))
      (:`else`))))

(event `TemporaryMessages`
  (if (`|EnumEquality` (`Widget.GetVisibility` (`self.WB_GameplayChat`)) "Hidden")
    (`Widget.SetVisibility` (`self.WB_GameplayChat`) "Visible")
    (`KismetSystemLibrary.Delay` 2.0)
    (`Widget.SetVisibility` (`self.WB_GameplayChat`) "Hidden")))

(fn `UserConstructionScript`)