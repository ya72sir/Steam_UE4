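; BP_SpawnerActor is a weapon pickup spawner that gives its configured weapon class to characters who touch it.
; The construction script previews that class's default static mesh on the pickup.
; On sphere overlap by a Character, it sends the class through an interface message.
; It then hides its meshes and spotlight and disables collision, restoring them after a short fixed delay to act as a respawn.
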(event `ToggleActiveWeapon`
  ;[1 1 1] Delete weapon on world and spawn to delay.
  (`SceneComponent.SetHiddenInGame` (`self.SpotLight`) true false)
  (`SceneComponent.SetHiddenInGame` (`self.StaticMeshWeapon`) true false)
  (`SceneComponent.SetHiddenInGame` (`self.StaticMesh`) true false)
  (`PrimitiveComponent.SetCollisionEnabled` (`self.Sphere`) "NoCollision")
  (`KismetSystemLibrary.Delay` 2.0)
  (`PrimitiveComponent.SetCollisionEnabled` (`self.Sphere`) "QueryAndPhysics")
  (`SceneComponent.SetHiddenInGame` (`self.StaticMeshWeapon`) false false)
  (`SceneComponent.SetHiddenInGame` (`self.StaticMesh`) false false)
  (`SceneComponent.SetHiddenInGame` (`self.SpotLight`) false false))

(event `self.Sphere.OnComponentBeginOverlap`
  (params (OverlappedComponent :type "PrimitiveComponent Object Reference") (OtherActor :type "Actor Object Reference") (OtherComp :type "PrimitiveComponent Object Reference") (OtherBodyIndex :type Integer) (bFromSweep :type Boolean) (SweepResult :type "HitResult Structure (by ref)"))
  (bind _ascharacter (cast `Character` OtherActor))
  (message `/Game/Sir/Core/Blueprints/Interfaces/BPI_Character.bpiSetWeapon` _ascharacter (`self.ClassWeaponForSpawn`))
  (`self.ToggleActiveWeapon`))

(fn `UserConstructionScript`
  (bind _classweaponforspawn (`self.ClassWeaponForSpawn`)
    (:`then`
      (`StaticMeshComponent.SetStaticMesh` (`self.StaticMeshWeapon`) (defaults `Object` _classweaponforspawn)))
    (:`else`)))