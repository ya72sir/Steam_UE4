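; Ammo projectile actor that damages Characters it overlaps and expires after a set lifespan.
; Its Sphere overlap ignores the Instigator, draws a red debug sphere at each other contact, then destroys the actor.
; Characters also receive point damage and a blood splash emitter at the projectile's location.
; The damage call passes a blank hit result and the projectile's world location as the hit direction.
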(event `self.ReceiveBeginPlay`
  (`self.SetLifeSpan` (`self.LifeSpan`)))

(event `self.Sphere.OnComponentBeginOverlap`
  (params (OverlappedComponent :type "PrimitiveComponent Object Reference") (OtherActor :type "Actor Object Reference") (OtherComp :type "PrimitiveComponent Object Reference") (OtherBodyIndex :type Integer) (bFromSweep :type Boolean) (SweepResult :type "HitResult Structure (by ref)"))
  (if (!= OtherActor (`self.Instigator`))
    (`KismetSystemLibrary.DrawDebugSphere` (`self.K2_GetActorLocation`) 25.0 12 (struct :`R` 1.0 :`A` 1.0) 5.0 3.0)
    (bind _ascharacter (cast `Character` OtherActor)
      (:`then`
        (`GameplayStatics.ApplyPointDamage` _ascharacter (`self.Damage`) (`self.K2_GetActorLocation`) (`GameplayStatics.MakeHitResult` false) null self)
        (`GameplayStatics.SpawnEmitterAtLocation` "/Game/Sir/Library/WeaponEffects/BloodImpact/psBloodSplash02.psBloodSplash02" (`self.K2_GetActorLocation`) (struct) (3.0 3.0 3.0))
        (`self.K2_DestroyActor`))
      (:`CastFailed`
        (`self.K2_DestroyActor`)))))

(fn `UserConstructionScript`)